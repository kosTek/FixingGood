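; BP_Beef is the beef food item, a child Blueprint that sets its type, initial status and energy thresholds for cooked and burnt on BeginPlay.
; While it is being grilled and received power reaches a minimum, Tick writes that power to the mesh material's BurntScale parameter.
; The FInterpTo on that value uses it as both current and target, so no smoothing occurs.
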(event EventBeginPlay
  (|CallParentFunction)
  (Variables|Default|SetType "NewEnumerator1")
  (Variables|Default|SetStatus "NewEnumerator1")
  (Variables|Default|SetEnergyRequiredForCooked 3.0)
  (Variables|Default|SetExtraEnergyRequiredForBurnt 1.5))

(event Collision|EventActorBeginOverlap
  (params (OtherActor :type Actor%20Object%20Reference))
  (|CallParentFunction OtherActor) ; This node is disabled and will not be called.\nDrag off pins to build functionality.
)

(event EventTick
  (params (DeltaSeconds :type Float%20%28single-precision%29))
  (bind _currentpowerreceived (Variables|Default|GetCurrentPowerReceived))
  (|CallParentFunction DeltaSeconds)
  (if (Variables|Default|GetIsBeingGrilled)
    (if (>= (Variables|Default|GetCurrentPowerReceived) 1.0)
      (Rendering|Material|SetScalarParameterValueonMaterials (Variables|Default|GetStaticMesh) "BurntScale" (Math|Interpolation|FInterpTo _currentpowerreceived _currentpowerreceived DeltaSeconds 0.5)))))

(fn ConstructionScript
  (|CallParentFunction))