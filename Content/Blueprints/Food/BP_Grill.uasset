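; BP_Grill is a grill that cooks BP_FoodParent items placed inside its Box trigger.
; It tracks overlapping food, starting grilling on entry and stopping it on exit.
; The item count sets grill power, switching from the base value to a fixed one at four or more items.
; Entering food receives the current power, while remaining items are only sent updated power when food leaves.
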(event OnComponentBeginOverlap(Box)
  (params (OverlappedComponent :type Primitive%20Component%20Object%20Reference) (OtherActor :type Actor%20Object%20Reference) (OtherComp :type Primitive%20Component%20Object%20Reference) (OtherBodyIndex :type Integer) (bFromSweep :type Boolean) (SweepResult :type Hit%20Result%20Structure%20%28by%20ref%29))
  (bind _overlappingobjects (Variables|Default|GetOverlappingObjects))
  (bind _asbp_food_parent (Utilities|Casting|CastToBP_FoodParent OtherActor))
  (Utilities|Array|Add _overlappingobjects OtherActor)
  (Variables|Default|SetNumber%20of%20Items (Utilities|Array|Length _overlappingobjects))
  (CallFunction|UpdatePowerOutput)
  (Default|StartGrilling _asbp_food_parent (Variables|Default|GetGrillPower) self))

(event OnComponentEndOverlap(Box)
  (params (OverlappedComponent :type Primitive%20Component%20Object%20Reference) (OtherActor :type Actor%20Object%20Reference) (OtherComp :type Primitive%20Component%20Object%20Reference) (OtherBodyIndex :type Integer))
  (bind _overlappingobjects (Variables|Default|GetOverlappingObjects))
  (bind _asbp_food_parent (Utilities|Casting|CastToBP_FoodParent OtherActor))
  (Default|StopGrilling _asbp_food_parent)
  (Utilities|Array|RemoveItem _overlappingobjects OtherActor)
  (Variables|Default|SetNumber%20of%20Items (Utilities|Array|Length _overlappingobjects))
  (CallFunction|UpdatePowerOutput)
  (for _array_element _overlappingobjects
    (bind _asbp_food_parent_2 (Utilities|Casting|CastToBP_FoodParent _array_element))
    (Default|UpdateGrillPower _asbp_food_parent_2 (Variables|Default|GetGrillPower) self)))

(event Custom|Update%20Power%20Output
  (if (>= (Variables|Default|GetNumber%20of%20Items) 4)
    (Variables|Default|SetGrillPower 0.025)
    (else
      (Variables|Default|SetGrillPower (/ (Variables|Default|GetBaseGrillPower) 1.0)))))

(event EventBeginPlay
  (Variables|Default|SetGrillPower (Variables|Default|GetBaseGrillPower)))

(event Collision|EventActorBeginOverlap
  (params (OtherActor :type Actor%20Object%20Reference)))

(event EventTick
  (params (DeltaSeconds :type Float%20%28single-precision%29)))

(fn ConstructionScript)