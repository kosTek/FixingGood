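; Base food actor that cooks and burns on a grill and can catch fire.
; Grill events set power and drive a looping one-second GrillFood timer that accumulates received energy.
; For one food Type, energy thresholds advance Status through cooked to burnt; other types only accumulate energy, at a boosted rate.
; Burnt status pauses the timer and attaches a fire particle system, which Extinguish removes once fire strength is depleted.
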(event Custom|Stop%20Grilling
  (Variables|Default|SetIsBeingGrilled false)
  (Class|KismetSystemLibrary|PauseTimer self "GrillFood"))

(event Custom|Update%20Grill%20Power
  (params (Grill%20Power :type Float%20%28single-precision%29) (Grill :type BP%20Grill%20Object%20Reference))
  (Variables|Default|SetGrillPower Grill%20Power)
  (Variables|Default|SetCurrentGrill Grill)
  (Utilities|Time|SetTimerbyFunctionName self "GrillFood" 1.0 true))

(event Custom|Extinguish
  (params (Strength :type Float%20%28single-precision%29))
  (if (Variables|Default|GetIsOnFire)
    (if (Variables|Default|GetIsOnFire)
      (bind _output_get (Variables|Default|SetFireStrength (- (Variables|Default|GetFireStrength) Strength)))
      (if (<= _output_get 0.0)
        (Components|DestroyComponent (Variables|Default|GetFireParticles))
        (Variables|Default|SetIsOnFire false)))))

(event Custom|Start%20Grilling
  (params (Grill%20Power :type Float%20%28single-precision%29) (Grill :type BP%20Grill%20Object%20Reference))
  (Variables|Default|SetIsBeingGrilled true)
  (Variables|Default|SetGrillPower Grill%20Power)
  (Variables|Default|SetCurrentGrill Grill)
  (Utilities|Time|SetTimerbyFunctionName self "GrillFood" 1.0 true))

(event Custom|Status%20Change
  (params (Status :type ENUM_FoodStatus%20Enum :default "NewEnumerator0"))
  (bind _output_get (Variables|Default|SetStatus Status))
  (if (Utilities|Enum|Equal(Enum) _output_get "NewEnumerator3")
    (Class|KismetSystemLibrary|PauseTimer self "GrillFood")
    (CallFunction|TriggerFireParticleSystem)))

(event EventBeginPlay
  (Variables|Default|SetType "NewEnumerator0")
  (Variables|Default|SetStatus "NewEnumerator0"))

(event Collision|EventActorBeginOverlap
  (params (OtherActor :type Actor%20Object%20Reference)))

(event EventTick
  (params (DeltaSeconds :type Float%20%28single-precision%29)))

(fn ConstructionScript)

(fn GrillFood
  (if (Utilities|Enum|Equal(Enum) (Variables|Default|GetType) "NewEnumerator1")
    (bind _output_get (Variables|Default|SetCurrentPowerReceived (+ (Variables|Default|GetGrillPower) (Variables|Default|GetCurrentPowerReceived))))
    (Variables|Default|SetMaterialFloat 1.0)
    (Variables|Default|SetMaterialFloat 0.0)
    (if (>= _output_get (Variables|Default|GetEnergyRequiredForCooked))
      (CallFunction|StatusChange "NewEnumerator2")
      (if (> (Variables|Default|GetCurrentPowerReceived) (+ (Variables|Default|GetEnergyRequiredForCooked) (Variables|Default|GetExtraEnergyRequiredForBurnt)))
        (CallFunction|StatusChange "NewEnumerator3")))
    (else
      (Variables|Default|SetCurrentPowerReceived (+ (* 3 (+ (Variables|Default|GetGrillPower) 0.1)) (Variables|Default|GetCurrentPowerReceived))))))

(fn TriggerFireParticleSystem
  (if (not (Variables|Default|GetIsOnFire))
    (bind _returnvalue (Niagara|SpawnSystemAttached "/Game/VFX/N_Fire_System.N_Fire_System" (Variables|Default|GetStaticMesh) "None" "0, 0, 0" "0, 0, 0" "KeepRelativeOffset" false))
    (Variables|Default|SetFireParticles _returnvalue)
    (Variables|Default|SetIsOnFire true)
    (Variables|Default|SetFireStrength 1e+02)))