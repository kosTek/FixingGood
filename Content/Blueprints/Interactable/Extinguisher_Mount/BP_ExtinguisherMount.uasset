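; BP_ExtinguisherMount is an interactable wall mount that hands out a fire extinguisher and takes it back.
; Grabbing it spawns a BP_Extinguisher near the mount and hides the display mesh.
; After a short delay, an extinguisher that begins overlapping the Box is destroyed and the display mesh reappears.
; The delay keeps the freshly spawned extinguisher from being immediately reabsorbed, though its flag is never reset after the first grab.
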(event OnComponentBeginOverlap(Box)
  (params (OverlappedComponent :type Primitive%20Component%20Object%20Reference) (OtherActor :type Actor%20Object%20Reference) (OtherComp :type Primitive%20Component%20Object%20Reference) (OtherBodyIndex :type Integer) (bFromSweep :type Boolean) (SweepResult :type Hit%20Result%20Structure%20%28by%20ref%29))
  (if (and (Variables|Default|GetCanDestroy) (not (Variables|Default|GetIsExtinguisherThere)))
    (bind _asbp_extinguisher (Utilities|Casting|CastToBP_Extinguisher OtherActor))
    (Actor|DestroyActor _asbp_extinguisher)
    (Rendering|SetVisibility (Variables|Default|GetSK_FireExtinguisher) true false)
    (Variables|Default|SetIsExtinguisherThere true)))

(event EventInteractGrab
  (if (Variables|Default|GetIsExtinguisherThere)
    (Game|SpawnActorfromClass "/Game/Blueprints/Interactable/Fire_Extinguisher/BP_Extinguisher.BP_Extinguisher_C" (Math|Transform|MakeTransform (+ (Transformation|GetWorldLocation (Variables|Default|GetSK_ExtinguisherMount)) "13.000000,0.000000,-20.000000") "0, 0, 0" "1,1,1") "Undefined" 0 0)
    (Rendering|SetVisibility (Variables|Default|GetSK_FireExtinguisher) false false)
    (Variables|Default|SetIsExtinguisherThere false)
    (Utilities|FlowControl|Delay 3.0)
    (Variables|Default|SetCanDestroy true)))

(event EventBeginPlay
  (Variables|Default|SetIsExtinguisherThere true)
  (Rendering|SetVisibility (Variables|Default|GetSK_FireExtinguisher) true false))

(fn ConstructionScript
  (|CallParentFunction))