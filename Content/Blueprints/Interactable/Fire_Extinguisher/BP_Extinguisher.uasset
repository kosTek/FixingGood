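; VR fire extinguisher that, while held, sprays on trigger press to put out BP_Beef actors.
; Pressing activates the Niagara particles and sets a blend space value; releasing stops them and resets it.
; The particle system exports data back to this actor, which sphere-traces at each particle position and calls Extinguish on any BP_Beef hit.
; Tick plays haptics on the holding hand while spraying.
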(event EventTriggerReleased
  (CallFunction|Deactivate))

(event EventTriggerPressed
  (CallFunction|Activate))

(event EventBeginPlay
  (Niagara|SetNiagaraVariable(Object) (Variables|Default|GetParticles) "User.ObjectCallback" self))

(event EventParticleData
  (params (Data :type Array%20of%20Basic%20Particle%20Data%20Structures) (NiagaraSystem :type Niagara%20System%20Object%20Reference))
  (for _array_element Data
    (bind _outhit (Collision|SphereTraceByChannel (.Position (Utilities|Struct|BreakBasicParticleData _array_element)) (.Position (Utilities|Struct|BreakBasicParticleData _array_element)) 5.0 "TraceTypeQuery1" false 0 "None"))
    (bind _asbp_beef (Utilities|Casting|CastToBP_Beef (.HitActor (Collision|BreakHitResult _outhit))))
    (Default|Extinguish _asbp_beef 0.4)))

(event EventTick
  (params (DeltaSeconds :type Float%20%28single-precision%29))
  (CallFunction|UpdateHaptics))

(fn ConstructionScript)

(fn Activate
  (if (Variables|/Game/VRTemplate/Blueprints/GrabComponent.GrabComponent_C|GetbIsHeld (Variables|Default|GetGrabComponentSnap))
    (Components|Activation|Activate (Variables|Default|GetParticles) false)
    (Variables|Default|SetIsExtinguishing true)
    (Variables|Default|SetBlendSpaceValue 1.0)))

(fn Deactivate
  (Components|Activation|Deactivate (Variables|Default|GetParticles))
  (Variables|Default|SetIsExtinguishing false)
  (Variables|Default|SetBlendSpaceValue 0.0))

(fn UpdateHaptics
  (if (Variables|Default|GetIsExtinguishing)
    (bind _returnvalue (Class|MagicLeapControllerFunctionLibrary|GetHandforMotionSource (Variables|/Script/HeadMountedDisplay.MotionControllerComponent|GetMotionSource (Variables|/Game/VRTemplate/Blueprints/GrabComponent.GrabComponent_C|GetMotionControllerRef (Variables|Default|GetGrabComponentSnap)))))
    (Class|PlayerController|PlayHapticEffect (Game|GetPlayerController 0) "/Game/VRTemplate/Haptics/FireExtinguisherHapticEffect.FireExtinguisherHapticEffect" _returnvalue 1.0 false)))