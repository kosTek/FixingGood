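; BP_Container_Parent is an interactable container that players open and close to pack products into.
; Interacting swaps between its opened and closed meshes, hiding the burger parts on close.
; While open, its InputBox overlap accepts one meth product and one finished burger, storing the burger's quality value.
; Accepted actors are destroyed and represented by pre-placed components that start hidden and become visible.
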(event OnComponentBeginOverlap(InputBox)
  (params (OverlappedComponent :type Primitive%20Component%20Object%20Reference) (OtherActor :type Actor%20Object%20Reference) (OtherComp :type Primitive%20Component%20Object%20Reference) (OtherBodyIndex :type Integer) (bFromSweep :type Boolean) (SweepResult :type Hit%20Result%20Structure%20%28by%20ref%29))
  ;[1 1 1] Put product inside of the container
  (if (not (Variables|Default|GetClosed?))
    (bind _asproduct_actor (Utilities|Casting|CastToProductActor OtherActor)
      (:then
        (if (and (Utilities|Enum|Equal(Enum) (Variables|/Script/FixingGood.ProductActor|GetType _asproduct_actor) "METH") (not (Variables|Default|GetHasMeth)))
          (Variables|Default|SetHasMeth true)
          (Rendering|SetVisibility (Variables|Default|GetMeth) true false)
          (Actor|DestroyActor _asproduct_actor)))
      (:CastFailed
        (bind _asbp_burger (Utilities|Casting|CastToBP_Burger OtherActor))
        (if (and (Variables|/Game/Blueprints/Burgers/Food/BP_Burger.BP_Burger_C|GetBurgerDone _asbp_burger) (not (Variables|Default|GetHasBurger)))
          (Variables|Default|SetHasBurger true)
          (Variables|Default|SetBurgerQuality (Variables|/Game/Blueprints/Burgers/Food/BP_Burger.BP_Burger_C|GetBurgerValue _asbp_burger))
          (Rendering|SetVisibility (Variables|Default|GetBurger) true false)
          (Rendering|SetVisibility (Variables|Default|GetBottom) true false)
          (Rendering|SetVisibility (Variables|Default|GetBeef) true false)
          (Actor|DestroyActor _asbp_burger))))))

(event Collision|EventActorBeginOverlap
  (params (OtherActor :type Actor%20Object%20Reference)))

(event EventTick
  (params (DeltaSeconds :type Float%20%28single-precision%29)))

(event EventInteractTrigger
  (bind _staticmesh (Variables|Default|GetStaticMesh))
  ;[1 1 1] Interaction
  (if (Variables|Default|GetClosed?)
    (Components|StaticMesh|SetStaticMesh _staticmesh (Variables|/Script/FixingGood.ContainerComponent|GetOpenedMesh (Variables|Default|GetContainer)))
    (Variables|Default|SetClosed? false)
    (else
      (Components|StaticMesh|SetStaticMesh _staticmesh (Variables|/Script/FixingGood.ContainerComponent|GetClosedMesh (Variables|Default|GetContainer)))
      (Variables|Default|SetClosed? true)
      (Rendering|SetVisibility (Variables|Default|GetBurger) false false)
      (Rendering|SetVisibility (Variables|Default|GetBottom) false false)
      (Rendering|SetVisibility (Variables|Default|GetBeef) false false))))

(event EventBeginPlay
  (Rendering|SetVisibility (Variables|Default|GetBurger) false false)
  (Rendering|SetVisibility (Variables|Default|GetMeth) false false)
  (Rendering|SetVisibility (Variables|Default|GetBottom) false false)
  (Rendering|SetVisibility (Variables|Default|GetBeef) false false))

(fn ConstructionScript)