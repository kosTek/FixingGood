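; BP_BinHoop is an actor that works as a bin hoop, scoring a point when something overlaps its Box trigger.
; An overlap calls IncreasePoints on the BP_UI_Hoop widget in its widget component and resets the points once they reach 100.
; A CanScore flag with a two-second delay blocks repeat scoring between overlaps.
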(event OnComponentBeginOverlap(Box)
  (params (OverlappedComponent :type Primitive%20Component%20Object%20Reference) (OtherActor :type Actor%20Object%20Reference) (OtherComp :type Primitive%20Component%20Object%20Reference) (OtherBodyIndex :type Integer) (bFromSweep :type Boolean) (SweepResult :type Hit%20Result%20Structure%20%28by%20ref%29))
  (if (Variables|Default|GetCanScore)
    (Variables|Default|SetCanScore false)
    (bind _asbp_ui_hoop (Utilities|Casting|CastToBP_UI_Hoop (UserInterface|GetWidget (Variables|Default|GetWidget))))
    (Default|IncreasePoints _asbp_ui_hoop)
    (if (>= (Variables|/Game/UI/Misc/BP_UI_Hoop.BP_UI_Hoop_C|GetPoints _asbp_ui_hoop) 100)
      (Default|ResetPoints _asbp_ui_hoop))
    (Utilities|FlowControl|Delay 2.0)
    (Variables|Default|SetCanScore true)))

(event EventBeginPlay)

(event Collision|EventActorBeginOverlap
  (params (OtherActor :type Actor%20Object%20Reference)))

(event EventTick
  (params (DeltaSeconds :type Float%20%28single-precision%29)))

(fn ConstructionScript)