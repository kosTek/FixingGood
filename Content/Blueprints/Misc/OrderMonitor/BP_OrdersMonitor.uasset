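; BP_OrdersMonitor is an in-world order screen that shows up to two orders, each either a burger alone or a burger with meth.
; It caches the UI_Ordering_Monitor from its widget component on BeginPlay.
; CreateOrder uses a reseeded random stream for a roughly even roll, toggles that side's icons and stores the order type.
; ClearOrder hides the icons and marks the slot empty.
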(event Custom|Clear%20Order
  (params (OrderNumber :type Integer))
  (if (== OrderNumber 1)
    (Widget|SetVisibility (Variables|/Game/UI/OrderMonitor/UI_Ordering_Monitor.UI_Ordering_Monitor_C|GetLeftBurger (Variables|Default|GetScreen)) "Hidden")
    (Widget|SetVisibility (Variables|/Game/UI/OrderMonitor/UI_Ordering_Monitor.UI_Ordering_Monitor_C|GetLeftMeth (Variables|Default|GetScreen)) "Hidden")
    (Variables|Default|SetOrderOne -1)
    (else
      (Widget|SetVisibility (Variables|/Game/UI/OrderMonitor/UI_Ordering_Monitor.UI_Ordering_Monitor_C|GetRightBurger (Variables|Default|GetScreen)) "Hidden")
      (Widget|SetVisibility (Variables|/Game/UI/OrderMonitor/UI_Ordering_Monitor.UI_Ordering_Monitor_C|GetRightMeth (Variables|Default|GetScreen)) "Hidden")
      (Variables|Default|SetOrderTwo -1))))

(event Custom|Create%20Order
  (params (OrderNumber :type Integer))
  (bind _screen (Variables|Default|GetScreen))
  (bind _screen_2 (Variables|Default|GetScreen))
  (bind _screen_3 (Variables|Default|GetScreen))
  (bind _screen_4 (Variables|Default|GetScreen))
  (bind _seed (Variables|Default|GetSeed))
  (bind _returnvalue (Class|KismetMathLibrary|RandomIntegerfromStream 100 _seed))
  (bind _leftburger (Variables|/Game/UI/OrderMonitor/UI_Ordering_Monitor.UI_Ordering_Monitor_C|GetLeftBurger _screen))
  (bind _leftmeth (Variables|/Game/UI/OrderMonitor/UI_Ordering_Monitor.UI_Ordering_Monitor_C|GetLeftMeth _screen_2))
  (bind _rightburger (Variables|/Game/UI/OrderMonitor/UI_Ordering_Monitor.UI_Ordering_Monitor_C|GetRightBurger _screen_4))
  (bind _rightmeth (Variables|/Game/UI/OrderMonitor/UI_Ordering_Monitor.UI_Ordering_Monitor_C|GetRightMeth _screen_3))
  (bind _returnvalue_2 (< _returnvalue 51))
  (if (== OrderNumber 1)
    (if _returnvalue_2
      (Widget|SetVisibility _leftburger "Visible")
      (Widget|SetVisibility _leftmeth "Hidden")
      (Variables|Default|SetOrderOne 1)
      (else
        (Widget|SetVisibility _leftburger "Visible")
        (Widget|SetVisibility _leftmeth "Visible")
        (Variables|Default|SetOrderOne 2)))
    (CallFunction|CreateNewSeed)
    (else
      ;[1 1 1] Order 2
      (if _returnvalue_2
        (Widget|SetVisibility _rightburger "Visible")
        (Widget|SetVisibility _rightmeth "Hidden")
        (Variables|Default|SetOrderTwo 1)
        (else
          (Widget|SetVisibility _rightburger "Visible")
          (Widget|SetVisibility _rightmeth "Visible")
          (Variables|Default|SetOrderTwo 2)))
      (CallFunction|CreateNewSeed))))

(event Custom|Create%20New%20Seed
  (Class|KismetMathLibrary|SeedRandomStream (Variables|Default|GetSeed)))

(event EventBeginPlay
  (bind _asui_ordering_monitor (Utilities|Casting|CastToUI_Ordering_Monitor (UserInterface|GetWidget (Variables|Default|GetWidget))))
  (Variables|Default|SetScreen _asui_ordering_monitor)
  (CallFunction|CreateNewSeed))

(fn ConstructionScript)