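; BP_BeefBasket is an interactable burger-station container that supplies beef.
; On the InteractGrab event it spawns a new BP_Beef actor at the world location of its Box component.
; There is no other active logic, and a vertical spawn offset is computed in the graph but left unconnected.
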(event EventBeginPlay
  (|CallParentFunction) ; This node is disabled and will not be called.\nDrag off pins to build functionality.
)

(event Collision|EventActorBeginOverlap
  (params (OtherActor :type Actor%20Object%20Reference))
  (|CallParentFunction OtherActor) ; This node is disabled and will not be called.\nDrag off pins to build functionality.
)

(event EventTick
  (params (DeltaSeconds :type Float%20%28single-precision%29))
  (|CallParentFunction DeltaSeconds) ; This node is disabled and will not be called.\nDrag off pins to build functionality.
)

(event EventInteractGrab
  (Game|SpawnActorfromClass "/Game/Blueprints/Food/BP_Beef.BP_Beef_C" (Math|Transform|MakeTransform (.location (Transformation|GetWorldTransform (Variables|Default|GetBox))) "0, 0, 0" "1,1,1") "Undefined" 0 0))

(fn ConstructionScript
  (|CallParentFunction))