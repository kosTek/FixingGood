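; BP_BreadBasket is an interactable basket actor that dispenses burger items when grabbed.
; Each InteractGrab alternates, via a FlipFlop boolean, between spawning a BP_Burger and a BP_BurgerIngredient initialized with the basket's FoodType.
; Both items spawn slightly above the basket's StaticMesh, inheriting its rotation and scale.
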(event EventBeginPlay
  (|CallParentFunction) ; This node is disabled and will not be called.\nDrag off pins to build functionality.
)

(event Collision|EventActorBeginOverlap
  (params (OtherActor :type Actor%20Object%20Reference))
  (|CallParentFunction OtherActor) ; This node is disabled and will not be called.\nDrag off pins to build functionality.
)

(event EventTick
  (params (DeltaSeconds :type Float%20%28single-precision%29))
  (|CallParentFunction DeltaSeconds) ; This node is disabled and will not be called.\nDrag off pins to build functionality.
)

(event EventInteractGrab
  (bind _self self)
  (bind _staticmesh (Variables|Default|GetStaticMesh _self))
  (bind _returnvalue (Transformation|GetWorldTransform _staticmesh))
  (bind _returnvalue_2 (+ (.location _returnvalue) "0, 0,23.500000"))
  (if (Variables|Default|GetFlipFlop)
    (Game|SpawnActorfromClass "/Game/Blueprints/Burgers/Food/BP_Burger.BP_Burger_C" (Math|Transform|MakeTransform _returnvalue_2 (.rotation _returnvalue) (.scale _returnvalue)) "Undefined" 0 0)
    (Variables|Default|SetFlipFlop false)
    (else
      (bind _returnvalue_3 (Game|SpawnActorfromClass "/Game/Blueprints/Burgers/Food/BP_BurgerIngredient.BP_BurgerIngredient_C" (Math|Transform|MakeTransform _returnvalue_2 (.rotation _returnvalue) (.scale _returnvalue)) "Undefined" 0 0))
      (Default|Setup _returnvalue_3 (Variables|Default|GetFoodType))
      (Variables|Default|SetFlipFlop true))))

(fn ConstructionScript
  (|CallParentFunction))