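; Burger actor that the player assembles by bringing ingredient actors into its collider, starting with all layers above the base hidden.
; A beef patty must come first, passing on its status and cooking power to set the burnt material parameter and burger value, which is zero if overcooked.
; Cheese, lettuce, two tomatoes and top bun must follow in order, each revealing its pre-placed component and destroying the ingredient, until the bun completes the burger.
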(event OnComponentBeginOverlap(Collider)
  (params (OverlappedComponent :type Primitive%20Component%20Object%20Reference) (OtherActor :type Actor%20Object%20Reference) (OtherComp :type Primitive%20Component%20Object%20Reference) (OtherBodyIndex :type Integer) (bFromSweep :type Boolean) (SweepResult :type Hit%20Result%20Structure%20%28by%20ref%29))
  (if (not (Variables|Default|GetBurgerDone))
    (bind _asbp_beef (Utilities|Casting|CastToBP_Beef OtherActor)
      (:then
        (if (not (Variables|Default|GetHasBeef))
          (Variables|Default|SetBeefStatus (Variables|/Game/Blueprints/Food/BP_FoodParent.BP_FoodParent_C|GetStatus _asbp_beef))
          (Rendering|Material|SetScalarParameterValueonMaterials (Variables|Default|GetBeef) "BurntScale" (Variables|/Game/Blueprints/Food/BP_FoodParent.BP_FoodParent_C|GetCurrentPowerReceived _asbp_beef))
          (if (> (Variables|/Game/Blueprints/Food/BP_FoodParent.BP_FoodParent_C|GetCurrentPowerReceived _asbp_beef) 3.5)
            (Variables|Default|SetBurgerValue 0.0)
            (else
              (Variables|Default|SetBurgerValue (* (/ (Variables|/Game/Blueprints/Food/BP_FoodParent.BP_FoodParent_C|GetCurrentPowerReceived _asbp_beef) 3e+02) 1e+02))))
          (Rendering|SetVisibility (Variables|Default|GetBeef) true false)
          (Actor|DestroyActor _asbp_beef)
          (Variables|Default|SetHasBeef true)))
      (:CastFailed
        (if (Variables|Default|GetHasBeef)
          (bind _asbp_burger_ingredient (Utilities|Casting|CastToBP_BurgerIngredient OtherActor))
          (if (Utilities|Enum|Equal(Enum) (Variables|/Game/Blueprints/Burgers/Food/BP_BurgerIngredient.BP_BurgerIngredient_C|GetIngredientType _asbp_burger_ingredient) "NewEnumerator0")
            (Rendering|SetVisibility (Variables|Default|GetCheese) true false)
            (Actor|DestroyActor _asbp_burger_ingredient)
            (Variables|Default|SetHasCheese true)
            (elif (and (Utilities|Enum|Equal(Enum) (Variables|/Game/Blueprints/Burgers/Food/BP_BurgerIngredient.BP_BurgerIngredient_C|GetIngredientType _asbp_burger_ingredient) "NewEnumerator2") (Variables|Default|GetHasCheese))
              (Rendering|SetVisibility (Variables|Default|GetLettuce) true false)
              (Actor|DestroyActor _asbp_burger_ingredient)
              (Variables|Default|SetHasLettuce true)
              (elif (Math|Boolean|ANDBoolean (Utilities|Enum|Equal(Enum) (Variables|/Game/Blueprints/Burgers/Food/BP_BurgerIngredient.BP_BurgerIngredient_C|GetIngredientType _asbp_burger_ingredient) "NewEnumerator1") (Variables|Default|GetHasCheese) (Variables|Default|GetHasLettuce) (not (Variables|Default|GetHasTomato1)))
                (Rendering|SetVisibility (Variables|Default|GetTomato_1) true false)
                (Actor|DestroyActor _asbp_burger_ingredient)
                (Variables|Default|SetHasTomato1 true)
                (elif (Math|Boolean|ANDBoolean (Utilities|Enum|Equal(Enum) (Variables|/Game/Blueprints/Burgers/Food/BP_BurgerIngredient.BP_BurgerIngredient_C|GetIngredientType _asbp_burger_ingredient) "NewEnumerator1") (Variables|Default|GetHasCheese) (Variables|Default|GetHasLettuce) (Variables|Default|GetHasTomato1) (not (Variables|Default|GetHasTomato2)))
                  (Rendering|SetVisibility (Variables|Default|GetTomato_2) true false)
                  (Actor|DestroyActor _asbp_burger_ingredient)
                  (Variables|Default|SetHasTomato2 true)
                  (elif (Math|Boolean|ANDBoolean (Utilities|Enum|Equal(Enum) (Variables|/Game/Blueprints/Burgers/Food/BP_BurgerIngredient.BP_BurgerIngredient_C|GetIngredientType _asbp_burger_ingredient) "NewEnumerator3") (Variables|Default|GetHasCheese) (Variables|Default|GetHasLettuce) (Variables|Default|GetHasTomato1) (Variables|Default|GetHasTomato2))
                    (Rendering|SetVisibility (Variables|Default|GetTopBun) true false)
                    (Actor|DestroyActor _asbp_burger_ingredient)
                    (Variables|Default|SetHasTopBun true)
                    (Variables|Default|SetBurgerDone true)))))))))))

(event EventBeginPlay
  (Rendering|SetVisibility (Variables|Default|GetBeef) false false)
  (Rendering|SetVisibility (Variables|Default|GetCheese) false false)
  (Rendering|SetVisibility (Variables|Default|GetLettuce) false false)
  (Rendering|SetVisibility (Variables|Default|GetTomato_1) false false)
  (Rendering|SetVisibility (Variables|Default|GetTomato_2) false false)
  (Rendering|SetVisibility (Variables|Default|GetTopBun) false false))

(fn ConstructionScript)