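; Burger ingredient Blueprint that represents one of cheese, tomato, salad or top bun, selected by its IngredientType.
; On BeginPlay it calls the parent, sets type, status and cook/burn energy thresholds, then runs Setup with its current IngredientType.
; The Setup event stores the given type and uses a chain of branches to assign the matching static mesh.
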(event Custom|Setup
  (params (Input :type ENUM_BurgerIngredientType%20Enum :default "NewEnumerator0"))
  (bind _output_get (Variables|Default|SetIngredientType Input))
  (if (Utilities|Enum|Equal(Enum) _output_get "NewEnumerator0")
    (Components|StaticMesh|SetStaticMesh (Variables|Default|GetStaticMesh) (Variables|/Script/FixingGood.BurgerIngredientComponent|GetCheeseMesh (Variables|Default|GetBurgerIngredient)))
    (elif (Utilities|Enum|Equal(Enum) (Variables|Default|GetIngredientType) "NewEnumerator1")
      (Components|StaticMesh|SetStaticMesh (Variables|Default|GetStaticMesh) (Variables|/Script/FixingGood.BurgerIngredientComponent|GetTomatoMesh (Variables|Default|GetBurgerIngredient)))
      (elif (Utilities|Enum|Equal(Enum) (Variables|Default|GetIngredientType) "NewEnumerator2")
        (Components|StaticMesh|SetStaticMesh (Variables|Default|GetStaticMesh) (Variables|/Script/FixingGood.BurgerIngredientComponent|GetSaladMesh (Variables|Default|GetBurgerIngredient)))
        (elif (Utilities|Enum|Equal(Enum) (Variables|Default|GetIngredientType) "NewEnumerator3")
          (Components|StaticMesh|SetStaticMesh (Variables|Default|GetStaticMesh) (Variables|/Script/FixingGood.BurgerIngredientComponent|GetTopBunMesh (Variables|Default|GetBurgerIngredient))))))))

(event EventBeginPlay
  (|CallParentFunction)
  (Variables|Default|SetType "NewEnumerator0")
  (Variables|Default|SetStatus "NewEnumerator0")
  (Variables|Default|SetEnergyRequiredForCooked 3.0)
  (Variables|Default|SetExtraEnergyRequiredForBurnt 0.0)
  (CallFunction|Setup (Variables|Default|GetIngredientType)))

(event Collision|EventActorBeginOverlap
  (params (OtherActor :type Actor%20Object%20Reference)))

(event EventTick
  (params (DeltaSeconds :type Float%20%28single-precision%29)))

(fn ConstructionScript)