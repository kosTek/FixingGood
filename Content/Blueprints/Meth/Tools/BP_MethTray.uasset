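; Tray actor for the meth production loop that collects liquid from an assigned flask and turns it into product actors.
; AssignFlask locks in one flask and its quality, while IncreaseMeth raises the amount and drives the fluid mesh's material parameter.
; Tick detects the empty flask and starts a timer for MakeMeth.
; MakeMeth spawns quality-tagged products at preset offsets, their count scaled by amount, then resets the tray.
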(event Custom|Assign%20Flask
  (params (Input :type BP%20Big%20Flask%20Object%20Reference))
  (if (not (Variables|Default|GetFlaskAssigned))
    (Utilities|IsValid Input
      (:Is%20Valid
        (bind _output_get (Variables|Default|SetFlask Input))
        (Variables|Default|SetFlaskAssigned true)
        (Variables|Default|SetMethQuality (Variables|/Game/Blueprints/Meth/Tools/BP_BigFlask.BP_BigFlask_C|GetQuality _output_get))))))

(event Custom|Increase%20Meth
  (bind _output_get (Variables|Default|SetMethAmount (+ (Variables|Default|GetMethAmount) 6.75)))
  (Rendering|Material|SetScalarParameterValueonMaterials (Variables|Default|GetSM_MetalTrayFluid) "MethAmount" _output_get)
  (CallFunction|ShowLiquid))

(event Custom|Make%20Meth
  (bind (_array_element _array_index) (Utilities|Array|ForEachLoopwithBreak (Variables|Default|GetSpawnPosition) :!label _label)
    (:LoopBody
      (if (== _array_index (.ReturnValue (Math|Float|Division(WholeandRemainder) (Variables|Default|GetMethAmount) 1687.5)))
        (goto _label Break)
        (else
          (bind _returnvalue (Game|SpawnActorfromClass "/Game/Blueprints/Meth/Product/BP_Product_Meth.BP_Product_Meth_C" (Math|Transform|MakeTransform (+ _array_element (Transformation|GetActorLocation self)) "0, 0, 0" "1,1,1") "Undefined" 0 0))
          (Default|SetQuality _returnvalue (Variables|Default|GetMethQuality)))))
    (:Completed
      (Variables|Default|SetFlaskAssigned false)
      (Variables|Default|SetFlask 0)
      (Variables|Default|SetIsMakingMeth false)
      (Variables|Default|SetMethAmount 0.0)
      (Variables|Default|SetMethQuality 0.0)
      (Variables|Default|SetShowMeth false)
      (Rendering|SetVisibility (Variables|Default|GetSM_MetalTrayFluid) false false))))

(event Custom|ShowLiquid
  (if (not (Variables|Default|GetShowMeth))
    (Rendering|SetVisibility (Variables|Default|GetSM_MetalTrayFluid) true false)
    (Variables|Default|SetShowMeth true)))

(event EventBeginPlay
  (Rendering|SetVisibility (Variables|Default|GetSM_MetalTrayFluid) false false))

(event Collision|EventActorBeginOverlap
  (params (OtherActor :type Actor%20Object%20Reference)))

(event EventTick
  (params (DeltaSeconds :type Float%20%28single-precision%29))
  (if (Math|Boolean|ANDBoolean (Variables|Default|GetFlaskAssigned) (Utilities|IsValid (Variables|Default|GetFlask)) (not (Variables|Default|GetIsMakingMeth)))
    (if (<= (Variables|/Game/Blueprints/Meth/Tools/BP_BigFlask.BP_BigFlask_C|GetCurrentLiquid (Variables|Default|GetFlask)) 0.0)
      (Variables|Default|SetIsMakingMeth true)
      (Utilities|Time|SetTimerbyEvent (delegate Custom|Make%20Meth) 3e+01))))

(fn ConstructionScript)