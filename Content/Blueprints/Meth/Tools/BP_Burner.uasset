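; BP_Burner is a toggleable burner tool that heats a BP_BigFlask placed above it.
; InteractTrigger flips between TurnOn and TurnOff, which set IsTurnedOn and activate or deactivate the Niagara effect.
; While on, Tick runs a short upward Visibility line trace from just above the actor.
; When the trace hits the flask's FIreTake component, it calls IncreaseFireEnergy on that flask every frame, without delta-time scaling.
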(event Custom|Turn%20on
  (Variables|Default|SetIsTurnedOn true)
  (Components|Activation|Activate (Variables|Default|GetNiagara) false))

(event Custom|Turn%20Off
  (Variables|Default|SetIsTurnedOn false)
  (Components|Activation|Deactivate (Variables|Default|GetNiagara)))

(event EventBeginPlay)

(event Collision|EventActorBeginOverlap
  (params (OtherActor :type Actor%20Object%20Reference)))

(event EventTick
  (params (DeltaSeconds :type Float%20%28single-precision%29))
  (bind _self self)
  (bind _returnvalue (Transformation|GetActorLocation _self))
  (bind _returnvalue_2 (+ _returnvalue "0, 0,25.000000"))
  (if (Variables|Default|GetIsTurnedOn)
    (bind _outhit (Collision|LineTraceByChannel _returnvalue_2 (+ _returnvalue_2 "0, 0,15.000000") "TraceTypeQuery1" false 0 "None"))
    (bind _asbp_big_flask (Utilities|Casting|CastToBP_BigFlask (.HitActor (Collision|BreakHitResult _outhit))))
    (if (== (Variables|/Game/Blueprints/Meth/Tools/BP_BigFlask.BP_BigFlask_C|GetFIreTake _asbp_big_flask) (.HitComponent (Collision|BreakHitResult _outhit)))
      (Default|IncreaseFireEnergy _asbp_big_flask))))

(event EventInteractTrigger
  (if (Variables|Default|GetIsTurnedOn)
    (CallFunction|TurnOff)
    (else
      (CallFunction|Turnon))))

(fn ConstructionScript)