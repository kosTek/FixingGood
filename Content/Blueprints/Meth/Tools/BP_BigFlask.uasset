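; BP_BigFlask is a meth-cooking flask that is filled with three ingredients, heated, then poured into a BP_MethTray.
; Ingredient events add volume up to capacity and update material parameters; enough fire energy readies the batch and calculates quality.
; Quality averages each ingredient's closeness to its ideal amount, penalizing overshoot.
; Tick uses roll to toggle the fluid and drain volume, line-tracing down to fill the tray, then resets state when empty.
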(event Custom|Handle%20Pouring
  (bind _self self)
  (bind _fluid (Variables|Default|GetFluid))
  (bind _returnvalue (Transformation|GetWorldLocation _fluid))
  (if (Variables|Default|GetIsPouring)
    (bind _outhit (Collision|LineTraceByChannel _returnvalue (+ _returnvalue "0.000000,0.000000,-2000.000000") "TraceTypeQuery1" false 0 "None"))
    (bind _asbp_meth_tray (Utilities|Casting|CastToBP_MethTray (.HitActor (Collision|BreakHitResult _outhit))))
    (if (== (Variables|/Game/Blueprints/Meth/Tools/BP_MethTray.BP_MethTray_C|GetTop _asbp_meth_tray) (.HitComponent (Collision|BreakHitResult _outhit)))
      (Utilities|IsValid (Variables|/Game/Blueprints/Meth/Tools/BP_MethTray.BP_MethTray_C|GetFlask _asbp_meth_tray)
        (:Is%20Valid
          _)
        (:Is%20Not%20Valid
          (Default|AssignFlask _asbp_meth_tray _self)))
      (if (== (Variables|/Game/Blueprints/Meth/Tools/BP_MethTray.BP_MethTray_C|GetFlask _asbp_meth_tray) _self)
        (Default|IncreaseMeth _asbp_meth_tray)))))

(event Custom|Increase%20Fire%20Energy
  ;[1 1 1] Pouring Liquid In
  (if (and (Variables|Default|GetReadyForFire) (not (Variables|Default|GetIsReady)))
    (bind _output_get (Variables|Default|SetFireEnergy (+ (Variables|Default|GetFireEnergy) 1.0)))
    (bind _output_get_2 (Variables|Default|SetIsReady (>= _output_get 1e+02)))
    (if _output_get_2
      (CallFunction|CalculateQuality)
      (Variables|Default|SetReadyForFire false))
    (else
      (Variables|Default|SetAtCapacity true)
      (Variables|Default|SetReadyForFire true))))

(event Custom|Increase%20Methylamine
  ;[1 1 1] Pouring Liquid In
  (if (not (Variables|Default|GetAtCapacity))
    (Variables|Default|SetMethylamine (+ (Variables|Default|GetMethylamine) 4.0))
    (CallFunction|IncreaseLiquidAmount 4.0)
    (Rendering|Material|SetScalarParameterValueonMaterials (Variables|Default|GetStaticMesh) "Methylamine" (Variables|Default|GetMethylamine))))

(event Custom|Increase%20Liquid%20Amount
  (params (Input :type Float%20%28single-precision%29))
  ;[1 1 1] Pouring Liquid In
  (Variables|Default|SetCurrentLiquid (+ (Variables|Default|GetCurrentLiquid) Input))
  (Variables|Default|SetIsEmpty false)
  (Rendering|Material|SetScalarParameterValueonMaterials (Variables|Default|GetStaticMesh) "Volume" (Variables|Default|GetCurrentLiquid))
  (if (>= (Variables|Default|GetCurrentLiquid) (Variables|Default|GetMaxLiquid))
    (Variables|Default|SetAtCapacity true)))

(event Custom|Increase%20Formate
  ;[1 1 1] Pouring Liquid In
  (if (not (Variables|Default|GetAtCapacity))
    (Variables|Default|SetMethylFormate (+ (Variables|Default|GetMethylFormate) 1.0))
    (CallFunction|IncreaseLiquidAmount 1.0)
    (Rendering|Material|SetScalarParameterValueonMaterials (Variables|Default|GetStaticMesh) "MethylFormate" (Variables|Default|GetMethylFormate))))

(event Custom|Calculate%20Quality
  (if (not (Variables|Default|GetHasQuality))
    (CallFunction|CalculateMythlamine)
    (CallFunction|CalculatePhenylacetone)
    (CallFunction|CalculateMethylFormate)
    (CallFunction|CalculateFinalQuality)))

(event Custom|Increase%20Phenylacetone
  ;[1 1 1] Pouring Liquid In
  (if (not (Variables|Default|GetAtCapacity))
    (Variables|Default|SetPhenylacetone (+ (Variables|Default|GetPhenylacetone) 1.0))
    (CallFunction|IncreaseLiquidAmount 1.0)
    (Rendering|Material|SetScalarParameterValueonMaterials (Variables|Default|GetStaticMesh) "Phenylacetone" (Variables|Default|GetPhenylacetone))))

(event Custom|Variable%20Purge
  (Variables|Default|SetMethylamine 0.0)
  (Variables|Default|SetPhenylacetone 0.0)
  (Variables|Default|SetMethylFormate 0.0)
  (Variables|Default|SetFireEnergy 0.0)
  (Variables|Default|SetCurrentLiquid 0.0)
  (Variables|Default|SetQuality 0.0)
  (Variables|Default|SetQualityTemp 0.0)
  (Variables|Default|SetIsPouring false)
  (Variables|Default|SetIsEmpty true)
  (Variables|Default|SetIsReady false)
  (Variables|Default|SetAtCapacity false))

(event EventBeginPlay)

(event Collision|EventActorBeginOverlap
  (params (OtherActor :type Actor%20Object%20Reference)))

(event EventTick
  (params (DeltaSeconds :type Float%20%28single-precision%29))
  (bind _self self)
  (bind _fluid (Variables|Default|GetFluid))
  (bind _returnvalue (Transformation|GetActorRotation _self))
  ;[1 1 1] Pouring Liquid out
  (if (and (not (Variables|Default|GetIsEmpty)) (Variables|Default|GetIsReady))
    (CallFunction|HandlePouring)
    (if (or (>= (.roll _returnvalue) 111.0) (<= (.roll _returnvalue) -91.0))
      (if (Variables|Default|GetIsPouring)
        (bind _output_get (Variables|Default|SetCurrentLiquid (- (Variables|Default|GetCurrentLiquid) 6.75)))
        (Rendering|Material|SetScalarParameterValueonMaterials (Variables|Default|GetStaticMesh) "Volume" _output_get)
        (if (<= _output_get 0.0)
          (Variables|Default|SetIsEmpty true)
          (Components|Activation|Deactivate (Variables|Default|GetFluid))
          (CallFunction|VariablePurge))
        (elif (not (Variables|Default|GetIsPouring))
          (Components|Activation|Activate _fluid false)
          (Variables|Default|SetIsPouring true)))
      (else
        (if (Variables|Default|GetIsPouring) :!label _label
          (Components|Activation|Deactivate _fluid)
          (Variables|Default|SetIsPouring false))))
    (else
      (goto _label))))

(fn ConstructionScript)

(fn CalculateMythlamine
  (if (> (Variables|Default|GetMethylamine) (Variables|Default|GetPerfectMethylamine))
    (Variables|Default|SetMethylamine (- (Variables|Default|GetPerfectMethylamine) (- (Variables|Default|GetMethylamine) (Variables|Default|GetPerfectMethylamine)))))
  (bind _output_get (Variables|Default|SetQualityTemp (+ (Variables|Default|GetQualityTemp) (/ (Variables|Default|GetMethylamine) (Variables|Default|GetPerfectMethylamine)))))
  (Development|PrintString (Utilities|String|ToString(Float) _output_get)))

(fn CalculatePhenylacetone
  (if (> (Variables|Default|GetPhenylacetone) (Variables|Default|GetPerfectPhenylacetone))
    (Variables|Default|SetPhenylacetone (- (Variables|Default|GetPerfectPhenylacetone) (- (Variables|Default|GetPhenylacetone) (Variables|Default|GetPerfectPhenylacetone)))))
  (bind _output_get (Variables|Default|SetQualityTemp (+ (Variables|Default|GetQualityTemp) (/ (Variables|Default|GetPhenylacetone) (Variables|Default|GetPerfectPhenylacetone)))))
  (Development|PrintString (Utilities|String|ToString(Float) _output_get) true true "(R=0.000000,G=1.000000,B=0.031100,A=1.000000)"))

(fn CalculateMethylFormate
  (if (> (Variables|Default|GetMethylFormate) (Variables|Default|GetPerfectMethylFormate))
    (Variables|Default|SetMethylFormate (- (Variables|Default|GetPerfectMethylFormate) (- (Variables|Default|GetMethylFormate) (Variables|Default|GetPerfectMethylFormate)))))
  (bind _output_get (Variables|Default|SetQualityTemp (+ (Variables|Default|GetQualityTemp) (/ (Variables|Default|GetMethylFormate) (Variables|Default|GetPerfectMethylFormate)))))
  (Development|PrintString (Utilities|String|ToString(Float) _output_get) true true "(R=0.147039,G=0.000000,B=0.500000,A=1.000000)"))

(fn CalculateFinalQuality
  (if (< (/ (Variables|Default|GetQualityTemp) 3.0) 0.0)
    (Variables|Default|SetQuality 0.0)
    (else
      (Variables|Default|SetQuality (/ (Variables|Default|GetQualityTemp) 3.0))))
  (Variables|Default|SetQualityTemp 0.0)
  (Development|PrintString (Utilities|String|ToString(Float) (Variables|Default|GetQuality)) true true "(R=1.000000,G=0.000000,B=0.072387,A=1.000000)"))