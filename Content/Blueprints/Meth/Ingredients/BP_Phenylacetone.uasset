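; BP_Phenylacetone is an interactable phenylacetone ingredient container that pours into a BP_BigFlask.
; Interacting toggles it open or closed by swapping the container mesh.
; Each tick, tilting the open container past roll thresholds activates the Fluid effect and drains its contents per frame until empty.
; While pouring, a downward line trace from the fluid increases the flask's phenylacetone when it hits the Intake component.
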(event Custom|Handle%20Pouring
  (bind _fluid (Variables|Default|GetFluid))
  (bind _returnvalue (Transformation|GetWorldLocation _fluid))
  (if (Variables|Default|GetIsPouring)
    (bind _outhit (Collision|LineTraceByChannel _returnvalue (+ _returnvalue "0.000000,0.000000,-2000.000000") "TraceTypeQuery1" false 0 "None"))
    (bind _asbp_big_flask (Utilities|Casting|CastToBP_BigFlask (.HitActor (Collision|BreakHitResult _outhit))))
    (if (== (Variables|/Game/Blueprints/Meth/Tools/BP_BigFlask.BP_BigFlask_C|GetIntake _asbp_big_flask) (.HitComponent (Collision|BreakHitResult _outhit)))
      (Default|IncreasePhenylacetone _asbp_big_flask))))

(event EventBeginPlay)

(event Collision|EventActorBeginOverlap
  (params (OtherActor :type Actor%20Object%20Reference))
  (|CallParentFunction OtherActor) ; This node is disabled and will not be called.\nDrag off pins to build functionality.
)

(event EventInteractTrigger
  (bind _staticmesh (Variables|Default|GetStaticMesh))
  (bind _container (Variables|Default|GetContainer))
  (if (Variables|Default|GetIsOpen)
    (Components|StaticMesh|SetStaticMesh _staticmesh (Variables|/Script/FixingGood.ContainerComponent|GetClosedMesh _container))
    (Variables|Default|SetIsOpen false)
    (else
      (Components|StaticMesh|SetStaticMesh _staticmesh (Variables|/Script/FixingGood.ContainerComponent|GetOpenedMesh _container))
      (Variables|Default|SetIsOpen true))))

(event EventTick
  (params (DeltaSeconds :type Float%20%28single-precision%29))
  (bind _self self)
  (bind _fluid (Variables|Default|GetFluid))
  (bind _returnvalue (Transformation|GetActorRotation _self))
  (|CallParentFunction DeltaSeconds)
  (if (and (not (Variables|Default|GetIsEmpty)) (Variables|Default|GetIsOpen))
    (CallFunction|HandlePouring)
    (if (or (>= (.roll _returnvalue) 111.0) (<= (.roll _returnvalue) -91.0))
      (if (Variables|Default|GetIsPouring)
        (bind _output_get (Variables|Default|SetLiquidLeft (- (Variables|Default|GetLiquidLeft) 1.0)))
        (if (<= _output_get 0.0)
          (Variables|Default|SetIsEmpty true)
          (Components|Activation|Deactivate (Variables|Default|GetFluid)))
        (elif (not (Variables|Default|GetIsPouring))
          (Components|Activation|Activate _fluid false)
          (Variables|Default|SetIsPouring true)))
      (else
        (if (Variables|Default|GetIsPouring) :!label _label
          (Components|Activation|Deactivate _fluid)
          (Variables|Default|SetIsPouring false))))
    (else
      (goto _label))))

(fn ConstructionScript
  (|CallParentFunction))