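; BP_Dispenser_Screen is the dispenser's screen actor, with a Box trigger that reacts to the VR player's proximity.
; When a VRPawn begins overlapping the Box, it turns on ShowDebug for the pawn's left and right WidgetInteraction components, and turns it off when the overlap ends.
; The debug display thus appears on both interaction components only while the pawn is inside the Box.
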(event OnComponentBeginOverlap(Box)
  (params (OverlappedComponent :type Primitive%20Component%20Object%20Reference) (OtherActor :type Actor%20Object%20Reference) (OtherComp :type Primitive%20Component%20Object%20Reference) (OtherBodyIndex :type Integer) (bFromSweep :type Boolean) (SweepResult :type Hit%20Result%20Structure%20%28by%20ref%29))
  (bind _asvrpawn (Utilities|Casting|CastToVRPawn OtherActor))
  (Variables|/Script/UMG.WidgetInteractionComponent|SetbShowDebug (Variables|/Game/VRTemplate/Blueprints/VRPawn.VRPawn_C|GetWidgetInteractionLeft _asvrpawn) true)
  (Variables|/Script/UMG.WidgetInteractionComponent|SetbShowDebug (Variables|/Game/VRTemplate/Blueprints/VRPawn.VRPawn_C|GetWidgetInteractionRight _asvrpawn) true))

(event OnComponentEndOverlap(Box)
  (params (OverlappedComponent :type Primitive%20Component%20Object%20Reference) (OtherActor :type Actor%20Object%20Reference) (OtherComp :type Primitive%20Component%20Object%20Reference) (OtherBodyIndex :type Integer))
  (bind _asvrpawn (Utilities|Casting|CastToVRPawn OtherActor))
  (Variables|/Script/UMG.WidgetInteractionComponent|SetbShowDebug (Variables|/Game/VRTemplate/Blueprints/VRPawn.VRPawn_C|GetWidgetInteractionLeft _asvrpawn) false)
  (Variables|/Script/UMG.WidgetInteractionComponent|SetbShowDebug (Variables|/Game/VRTemplate/Blueprints/VRPawn.VRPawn_C|GetWidgetInteractionRight _asvrpawn) false))

(event EventBeginPlay)

(event Collision|EventActorBeginOverlap
  (params (OtherActor :type Actor%20Object%20Reference)))

(event EventTick
  (params (DeltaSeconds :type Float%20%28single-precision%29)))

(fn ConstructionScript)